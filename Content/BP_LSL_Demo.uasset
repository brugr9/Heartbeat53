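; Demo actor that connects to an MQTT broker to show received heart-rate data on a heart mesh and text display.
; BeginPlay connects and enters standby with spinning heart and blinking text; subscribed messages pass as JSON to HeartbeatUpdate, and EndPlay tears down.
; HeartbeatUpdate is empty here; nodes setting HR text and RR-based pulse timeline rate sit unwired.
; Timer-chained Testing events feed sample JSON, then cycle standby and deactivate.
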(event `self.ReceiveBeginPlay`
  ;[0 1 0.4 0.5] Startup Messaging
  (bind _returnvalue (`self.GetOrCreateClient_WithProjectURL` null))
  (bind (_output_get _output_get_2) (set `self.MyClient` null _returnvalue))
  (`self.Connect` _output_get_2 (delegate `OnConnect`))
  (`self.HeartbeatStandBy`))

(event `HeartbeatStandby`
  ;[1 0 0] Heartbeat
  ;;[1 1 1] Heartbeat Standby
  (`self.HeartbeatReset`)
  (`ActorComponent.Activate` (`self.RotatingMovement`) false)
  (bind _returnvalue (`KismetSystemLibrary.K2_SetTimerDelegate` (delegate `TextRenderBlink`) 0.5 true))
  (set `self.TextRenderVisibilityTimer` _returnvalue))

(event `OnConnect`
  (params (ReturnCode :type Byte :default 0))
  ;[0 1 0.4 0.5] Startup Messaging
  (switch `|SwitchEnum` ReturnCode
    (:`Accepted`
      (bind _returnvalue (`self.Subscribe` (`.MyClient` (`self.MyClient`)) (`self.MyTopic`) 0 :!label _label))
      (bind (_output_get _output_get_2) (set `self.MySubscription` null _returnvalue))
      (`self.SetOnMessageHandler` _output_get_2 (delegate `OnMessage`)))
    (:`RefusedProtocolVersion`
      (`KismetSystemLibrary.PrintString` (`|GetEnumeratorNameAsString` ReturnCode) false :!label _label_2)
      (`self.Teardown Messaging`))
    (:`RefusedIdentifierRejected`
      (goto _label_2))
    (:`AlreadyConnected`
      (goto _label))))

(event `TextRenderBlink`
  ;[1 0 0] Heartbeat
  ;;[1 1 1] Heartbeat Standby
  (bind _isa (`/Engine/EditorBlueprintResources/StandardMacros.FlipFlop`)
    (:`A`
      _)
    (:`B`
      _))
  (`SceneComponent.SetVisibility` (`Actor.RootComponent` (`self.TextRender`)) _isa false))

(event `OnMessage`
  (params (Message :type " Structure (by ref)"))
  ;[0 1 0.4 0.5] Startup Messaging
  (`KismetSystemLibrary.PrintString` (`self.GetPayloadString` Message) false)
  (`self.HeartbeatUpdate` (`self.GetPayloadJson` (`.MySubscription` (`self.MySubscription`)) Message)))

(event `HeartbeatUpdate`
  (params (JsonObject :type "JsonObjectWrapper Structure"))
  ;[1 0 0] Heartbeat
  ;;[1 1 1] Heartbeat Update
)

(event `Teardown Messaging`
  (bind (_myclient _myclient_2) (`self.MyClient`))
  ;[1 0 1 0.5] Teardown Messaging
  (`self.Unsubscribe` _myclient_2 (`self.MyTopic`))
  (`self.HeartbeatDeactivate`)
  (`self.Disconnect` _myclient_2 (delegate `OnDisconnect`)))

(event `OnDisconnect`
  ;[1 0 1 0.5] Teardown Messaging
  (`KismetSystemLibrary.PrintString` "MQTT Client disconnected" false))

(event `self.ReceiveEndPlay`
  (params (EndPlayReason :type "EEndPlayReason Enum" :default "Destroyed"))
  ;[1 0 1 0.5] Teardown Messaging
  (`self.Teardown Messaging`))

(event `HeartbeatDeactivate`
  ;[1 0 0] Heartbeat
  ;;[1 1 1] Heartbeat Deactivate
  (`self.HeartbeatReset`)
  ;;[1 1 1] Heartbeat Update
  ;;;[0 0.7 1] Field RR: Timeline
  (`/Engine/EditorBlueprintResources/StandardMacros.DoOnce` false :!via `Reset`
    (:`Completed`
      (`self.HeartbeatReset`)
      (bind (_direction _alpha) (`Timeline|HeartbeatTimeline` :!via `PlayFromStart`)
        (:`Update`
          (`SceneComponent.SetRelativeScale3D` (`self.HeartMesh`) (`KismetMathLibrary.VLerp` (1.0 1.0 1.0) (2.0 2.0 2.0) _alpha)))))))

(event `Testing01`
  ;[1 1 0] Testing
  (`KismetSystemLibrary.K2_SetTimerDelegate` (delegate `Testing02`) 5.0)
  (bind (_outjsonobject _returnvalue) (`self.FromString` "{ \n  \"clientId\": \"MyPSL-01\", \n  \"deviceId\": \"12345678\", \n  \"sessionId\": 1234567890, \n  \"timeStamp\": 1235678901234, \n  \"hr\": 124, \n  \"rr\": [ \n    484, 555 \n  ] \n}"))
  (if _returnvalue
    (`self.HeartbeatUpdate` _outjsonobject)))

(event `Testing02`
  ;[1 1 0] Testing
  (`KismetSystemLibrary.K2_SetTimerDelegate` (delegate `Testing03`) 5.0)
  (`self.HeartbeatStandBy`))

(event `HeartbeatReset`
  (bind _textrender (`self.TextRender`))
  ;[1 0 0] Heartbeat
  ;;[1 1 1] Helper Event: Heartbeat Reset
  (`TimelineComponent.Stop` (`self.HeartbeatTimeline`))
  (`SceneComponent.SetRelativeScale3D` (`self.HeartMesh`) (1.0 1.0 1.0))
  (`ActorComponent.Deactivate` (`self.RotatingMovement`))
  (`SceneComponent.K2_SetWorldRotation` :`self` (`self.HeartMesh`))
  (`KismetSystemLibrary.K2_ClearAndInvalidateTimerHandle` (`self.TextRenderVisibilityTimer`))
  (`SceneComponent.SetVisibility` (`Actor.RootComponent` _textrender) true false)
  (`TextRenderComponent.K2_SetText` (`TextRenderActor.TextRender` _textrender) "HR"))

(event `Testing03`
  ;[1 1 0] Testing
  (`self.HeartbeatDeactivate`))

(fn `UserConstructionScript`)