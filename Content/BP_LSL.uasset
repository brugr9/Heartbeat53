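; BP_LSL is a test relay for Lab Streaming Layer (LSL) data, with an inlet and an outlet component.
; Inlet float updates print their first channel and push it to the outlet as a single-element string sample.
; String updates print their first element and pass the whole array through to the same outlet.
; Stream exceptions from the inlet are printed, while BeginPlay and Tick stay empty.
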(event `self.ReceiveBeginPlay`)

(event `self.ReceiveTick`
  (params (DeltaSeconds :type "Float (single-precision)")))

(event `self.LSLInlet.OnStreamCaughtException`
  (params (ErrorString :type String))
  (`KismetSystemLibrary.PrintString` ErrorString))

(event `self.LSLInlet.OnStreamUpdatedFloat`
  (params (FloatArray :type "Array of Float (single-precision) (by ref)") (DeltaSeconds :type "Float (single-precision)"))
  (bind _returnvalue (`KismetStringLibrary.Conv_DoubleToString` (`|GetArrayItem` FloatArray)))
  (`KismetSystemLibrary.PrintString` _returnvalue)
  (`LSLOutletComponent.PushSampleString` (`self.LSLOutlet`) (`|MakeArray` _returnvalue)))

(event `self.LSLInlet.OnStreamUpdatedString`
  (params (StringArray :type "Array of String (by ref)") (DeltaSeconds :type "Float (single-precision)"))
  (`KismetSystemLibrary.PrintString` (`|GetArrayItem` StringArray))
  (`LSLOutletComponent.PushSampleString` (`self.LSLOutlet`) StringArray))

(fn `UserConstructionScript`)