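; Heartbeat display actor with a heart mesh and HR text, plus Lab Streaming Layer inlet and outlet.
; Standby, entered on begin play or stream error, rotates the heart and blinks the label.
; HeartbeatUpdate sets HR text and drives a scale-pulse timeline at an RR-derived rate, but its only call never runs.
; Incoming samples' first float is currently just printed and echoed to the outlet, as are error strings.
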(event `self.ReceiveBeginPlay`
  (`self.HeartbeatStandby`))

(event `self.ReceiveTick`
  (params (DeltaSeconds :type "Float (single-precision)")))

(event `self.LSLInlet.OnStreamCaughtException`
  (params (ErrorString :type String))
  (`self.HeartbeatStandby`)
  (`LSLOutletComponent.PushSampleString` (`self.LSLOutlet`) (`|MakeArray` ErrorString)))

(event `self.LSLInlet.OnStreamUpdatedFloat`
  (params (FloatArray :type "Array of Float (single-precision) (by ref)") (DeltaSeconds :type "Float (single-precision)"))
  (bind _returnvalue (`KismetStringLibrary.Conv_DoubleToString` (`|GetArrayItem` FloatArray)))
  (`LSLOutletComponent.PushSampleString` (`self.LSLOutlet`) (`|MakeArray` _returnvalue))
  (`KismetSystemLibrary.PrintString` _returnvalue))

(event `HeartbeatReset`
  (bind _textrender (`self.TextRender`))
  ;[1 1 1] Helper Event: Heartbeat Reset
  (`SceneComponent.SetRelativeScale3D` (`self.HeartMesh`) (1.0 1.0 1.0))
  (`ActorComponent.Deactivate` (`self.RotatingMovement`))
  (`SceneComponent.K2_SetWorldRotation` :`self` (`self.HeartMesh`))
  (`KismetSystemLibrary.K2_ClearAndInvalidateTimerHandle` (`self.TextRenderVisibilityTimer`))
  (`SceneComponent.SetVisibility` (`Actor.RootComponent` _textrender) true false)
  (`TextRenderComponent.K2_SetText` (`TextRenderActor.TextRender` _textrender) "HR"))

(event `HeartbeatStandby`
  ;[1 1 1] Heartbeat Standby
  (`self.HeartbeatReset`)
  (`ActorComponent.Activate` (`self.RotatingMovement`) false)
  (bind _returnvalue (`KismetSystemLibrary.K2_SetTimerDelegate` (delegate `TextRenderBlink`) 0.5 true))
  (set `self.TextRenderVisibilityTimer` _returnvalue))

(event `TextRenderBlink`
  ;[1 1 1] Heartbeat Standby
  (bind _isa (`/Engine/EditorBlueprintResources/StandardMacros.FlipFlop`)
    (:`A`
      _)
    (:`B`
      _))
  (`SceneComponent.SetVisibility` (`Actor.RootComponent` (`self.TextRender`)) _isa false))

(event `HeartbeatDeactivate`
  ;[1 1 1] Heartbeat Deactivate
  (`self.HeartbeatReset`)
  (goto _label :!via `Reset`))

(event `HeartbeatUpdate`
  (params (RR :type "Float (double-precision)") (HR :type Integer))
  ;[1 1 1] Heartbeat Update
  ;;[0 0.7 1] RR: Timeline
  (`|ExecutionSequence`
    (:`then_0`
      (`/Engine/EditorBlueprintResources/StandardMacros.DoOnce` false :!label _label
        (:`Completed`
          (`self.HeartbeatReset`)
          (bind (_direction _alpha) (`Timeline|HeartbeatTimeline` :!via `PlayFromStart`)
            (:`Update`
              (`SceneComponent.SetRelativeScale3D` (`self.HeartMesh`) (`KismetMathLibrary.VLerp` (1.0 1.0 1.0) (2.0 2.0 2.0) _alpha)))))))
    (:`then_1`
      (`TimelineComponent.SetPlayRate` (`self.HeartbeatTimeline`) (/ 1000.0 RR)))
    (:`then_2`
      ;;[0 0.7 1] HR
      (`TextRenderComponent.K2_SetText` (`TextRenderActor.TextRender` (`self.TextRender`)) (`KismetTextLibrary.Conv_IntToText` HR)))))

(fn `UserConstructionScript`
  (set `LSLInletComponent.StreamName` (`self.InletStreamName`) (`self.LSLInlet`)))